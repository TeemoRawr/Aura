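; GA_RangedAttack is an enemy gameplay ability that fires a projectile at the avatar's current combat target.
; On activation it turns the avatar to face the target through CombatInterface and plays a random tagged attack montage.
; A one-shot gameplay event matching the montage's tag triggers the projectile spawn from the tagged socket with a fixed pitch override, then ends the ability.
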(event `self.K2_ActivateAbility`
  (bind _returnvalue (`self.GetAvatarActorFromActorInfo`))
  (bind _returnvalue_2 (message `EnemyInterface.GetCombatTarget` _returnvalue))
  (bind _output_get (set `self.CombatTarget` _returnvalue_2))
  (bind _ascombat_interface (cast `CombatInterface` _returnvalue))
  (`CombatInterface.UpdateFacingTarget` _ascombat_interface (`Actor.K2_GetActorLocation` _output_get))
  (bind _returnvalue_3 (`CombatInterface.GetAttackMontages` _ascombat_interface))
  (bind _output_get_2 (set `self.RandomTaggedMontage` (`KismetArrayLibrary.Array_Random` _returnvalue_3)))
  (bind (_montage _montagetag _sockettag) (break `TaggedMontage` _output_get_2))
  (`AbilityTask_PlayMontageAndWait.CreatePlayMontageAndWaitProxy` "None" _montage 1.0 "None" false
    (:`then`
      (`AbilityTask_WaitGameplayEvent.WaitGameplayEvent` _montagetag null true
        (:`EventReceived`
          (`self.SpawnProjectile` (`Actor.K2_GetActorLocation` (`self.CombatTarget`)) _sockettag true 15.0)
          (`self.K2_EndAbility`))))))