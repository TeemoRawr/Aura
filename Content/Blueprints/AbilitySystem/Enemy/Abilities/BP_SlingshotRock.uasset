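; BP_SlingshotRock is a rock actor under enemy abilities, likely a slingshot projectile, that handles the spin of its rock mesh.
; When an actor overlap begins, it picks one random signed rate and copies it to yaw, pitch and roll.
; Tick applies those rates, scaled by delta time, as local rotation to RockMesh.
; The graph contains no movement or damage logic, and BeginPlay is unused.
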(event `self.ReceiveActorBeginOverlap`
  (params (OtherActor :type "Actor Object Reference"))
  (bind _output_get (set `self.YawRotationRate` (`KismetMathLibrary.RandomFloatInRange` -500.0 500.0)))
  (bind _output_get_2 (set `self.PitchRotationRate` _output_get))
  (set `self.RollRotationRate` _output_get_2))

(event `self.ReceiveTick`
  (params (DeltaSeconds :type "Float (single-precision)"))
  (`SceneComponent.K2_AddLocalRotation` (`self.RockMesh`) (`KismetMathLibrary.MakeRotator` (* DeltaSeconds (`self.RollRotationRate`)) (* DeltaSeconds (`self.PitchRotationRate`)) (* DeltaSeconds (`self.YawRotationRate`))) false false))

(fn `UserConstructionScript`)