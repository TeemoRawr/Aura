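; Enemy melee attack ability that turns the avatar toward its combat target and plays a random tagged attack montage.
; When the montage's tagged gameplay event arrives, it searches a small sphere at that attack's combat socket for live, non-friendly players and damages them.
; Any hit fires one MeleeImpact gameplay cue at the socket.
; The ability then ends without stopping the montage, and also ends on interruption or cancellation.
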(event `self.K2_ActivateAbility`
  (bind _returnvalue (`self.GetAvatarActorFromActorInfo`))
  (bind _returnvalue_2 (`self.GetAvatarActorFromActorInfo`))
  (bind (_randomtaggedmontage_montage _randomtaggedmontage_montagetag) (break `TaggedMontage` (`self.RandomTaggedMontage`)))
  (set `self.HasHitTarget` false)
  (bind _returnvalue_3 (message `EnemyInterface.GetCombatTarget` _returnvalue))
  (bind _output_get (set `self.CombatTarget` _returnvalue_3))
  (bind _ascombat_interface (cast `CombatInterface` _returnvalue))
  (`CombatInterface.UpdateFacingTarget` _ascombat_interface (`Actor.K2_GetActorLocation` _output_get))
  (bind _returnvalue_4 (`CombatInterface.GetAttackMontages` _ascombat_interface))
  (bind _output_get_2 (set `self.RandomTaggedMontage` (`KismetArrayLibrary.Array_Random` _returnvalue_4)))
  (bind (_montage _montagetag _sockettag) (break `TaggedMontage` _output_get_2))
  (`AbilityTask_PlayMontageAndWait.CreatePlayMontageAndWaitProxy` "None" _montage 1.0 "None" false
    (:`then`
      (`AbilityTask_WaitGameplayEvent.WaitGameplayEvent` _montagetag null
        (:`EventReceived`
          (bind _returnvalue_5 (message `CombatInterface.GetCombatSocketLocation` _returnvalue_2 _sockettag))
          (set `self.CombatSocketLocation` _returnvalue_5)
          (bind _outoverlappingactors (`AuraAbilitySystemLibrary.GetLivePlayersWithinRadius` self (`|MakeArray` _returnvalue_2) 45.0 (`self.CombatSocketLocation`)))
          (for _array_element _outoverlappingactors
            (bind _returnvalue_6 (`AuraAbilitySystemLibrary.IsNotFriend` (`self.GetAvatarActorFromActorInfo`) _array_element))
            (if _returnvalue_6
              (`AuraAbilitySystemLibrary.ApplyDamageEffect` (`self.MakeDamageParamsFromClassDefaults` _array_element))
              (set `self.HasHitTarget` true)))
          (if (`self.HasHitTarget`)
            (`self.K2_ExecuteGameplayCueWithParams` (struct :`TagName` "GameplayCue.MeleeImpact") (`AbilitySystemBlueprintLibrary.MakeGameplayCueParameters` 0.0 0.0 (struct) (struct) (struct) (`BlueprintGameplayTagLibrary.MakeGameplayTagContainerFromTag` _randomtaggedmontage_montagetag) (struct) (`self.CombatSocketLocation`) (0.0 0.0 0.0) null (`self.GetAvatarActorFromActorInfo`) (`self.CombatTarget`))))
          (`self.K2_EndAbility`))))
    (:`OnInterrupted`
      (`self.K2_EndAbility` :!label _label))
    (:`OnCancelled`
      (goto _label))))