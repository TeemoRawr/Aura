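; BP_AuraCharacter is the Aura character Blueprint, adding facing, occluder fade and shock-loop hooks.
; UpdateFacingTarget feeds a location into Motion Warping as the FacingTarget warp target.
; A Box component's overlaps send fade-out on entry and fade-in on exit to actors implementing BI_Fade.
; SetinShockLoop stores the InShockLoop flag.
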(event `CombatInterface.UpdateFacingTarget`
  (params (Location :type "Vector Structure"))
  (`MotionWarpingComponent.AddOrUpdateWarpTargetFromLocation` (`self.MotionWarping`) "FacingTarget" Location))

(event `self.Box.OnComponentBeginOverlap`
  (params (OverlappedComponent :type "PrimitiveComponent Object Reference") (OtherActor :type "Actor Object Reference") (OtherComp :type "PrimitiveComponent Object Reference") (OtherBodyIndex :type Integer) (bFromSweep :type Boolean) (SweepResult :type "HitResult Structure (by ref)"))
  (if (`KismetSystemLibrary.DoesImplementInterface` OtherActor "/Game/Blueprints/Actor/FadeActor/BI_Fade.BI_Fade_C")
    (message `/Game/Blueprints/Actor/FadeActor/BI_Fade.FadeOut` OtherActor)))

(event `self.Box.OnComponentEndOverlap`
  (params (OverlappedComponent :type "PrimitiveComponent Object Reference") (OtherActor :type "Actor Object Reference") (OtherComp :type "PrimitiveComponent Object Reference") (OtherBodyIndex :type Integer))
  (if (`KismetSystemLibrary.DoesImplementInterface` OtherActor "/Game/Blueprints/Actor/FadeActor/BI_Fade.BI_Fade_C")
    (message `/Game/Blueprints/Actor/FadeActor/BI_Fade.FadeIn` OtherActor)))

(event `CombatInterface.SetInShockLoop`
  (params (bInLoop :type Boolean))
  (set `self.InShockLoop` bInLoop))

(fn `UserConstructionScript`)