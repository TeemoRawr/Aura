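; BP_EnemyBase is a base enemy character Blueprint that handles spawn, facing and dissolve presentation.
; On BeginPlay a timeline animates the mesh's uniform scale as a spawn effect.
; UpdateFacingTarget feeds a location to Motion Warping as the FacingTarget warp target.
; Two events run separate timelines that drive the Dissolve parameter on supplied dynamic material instances, one for the weapon.
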(event `self.ReceiveBeginPlay`
  (bind (_direction _scaletrack) (`Timeline|SpawnTimeline`)
    (:`Update`
      (`SceneComponent.SetRelativeScale3D` (`self.Mesh`) (`KismetMathLibrary.MakeVector` _scaletrack _scaletrack _scaletrack)))))

(event `CombatInterface.UpdateFacingTarget`
  (params (Location :type "Vector Structure"))
  (`MotionWarpingComponent.AddOrUpdateWarpTargetFromLocation` (`self.MotionWarping`) "FacingTarget" Location))

(event `self.StartDissolveTimeline`
  (params (DynamicMaterialInstance :type "MaterialInstanceDynamic Object Reference"))
  (bind (_direction _disolvetrack) (`Timeline|Disolve Timeline`)
    (:`Update`
      (`MaterialInstanceDynamic.SetScalarParameterValue` DynamicMaterialInstance "Dissolve" _disolvetrack))))

(event `self.StartWeaponDissolveTimeline`
  (params (DynamicMaterialInstance :type "MaterialInstanceDynamic Object Reference"))
  (bind (_direction _weapondisolvetrack) (`Timeline|Timeline`)
    (:`Update`
      (`MaterialInstanceDynamic.SetScalarParameterValue` DynamicMaterialInstance "Dissolve" _weapondisolvetrack))))

(fn `UserConstructionScript`)