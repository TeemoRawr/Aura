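; Enemy melee attack Gameplay Ability that turns the avatar toward its combat target and plays a random tagged attack montage from the combat interface.
; When the gameplay event matching the montage's tag arrives, it finds live players in a small sphere around that tag's combat socket.
; It damages each non-friendly one, then ends.
; An interrupted or cancelled montage also ends the ability.
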(event `self.K2_ActivateAbility`
  (bind _returnvalue (`self.GetAvatarActorFromActorInfo`))
  (bind _returnvalue_2 (`self.GetAvatarActorFromActorInfo`))
  (bind _returnvalue_3 (message `EnemyInterface.GetCombatTarget` _returnvalue))
  (bind _output_get (set `self.CombatTarget` _returnvalue_3))
  (bind _ascombat_interface (cast `CombatInterface` _returnvalue))
  (`CombatInterface.UpdateFacingTarget` _ascombat_interface (`Actor.K2_GetActorLocation` _output_get))
  (bind _returnvalue_4 (`CombatInterface.GetAttackMontages` _ascombat_interface))
  (bind _output_get_2 (set `self.RandomTaggedMontage` (`KismetArrayLibrary.Array_Random` _returnvalue_4)))
  (bind (_montage _montagetag) (break `TaggedMontage` _output_get_2))
  (`AbilityTask_PlayMontageAndWait.CreatePlayMontageAndWaitProxy` "None" _montage 1.0 "None" false
    (:`then`
      (`AbilityTask_WaitGameplayEvent.WaitGameplayEvent` _montagetag null
        (:`EventReceived`
          (bind _returnvalue_5 (message `CombatInterface.GetCombatSocketLocation` _returnvalue_2 _montagetag))
          (bind _outoverlappingactors (`AuraAbilitySystemLibrary.GetLivePlayersWithinRadius` self (`|MakeArray` _returnvalue_2) 45.0 _returnvalue_5))
          (for _array_element _outoverlappingactors
            (bind _returnvalue_6 (`AuraAbilitySystemLibrary.IsNotFriend` (`self.GetAvatarActorFromActorInfo`) _array_element))
            (if _returnvalue_6
              (`self.CauseDamage` _array_element)))
          (`self.K2_EndAbility`))))
    (:`OnInterrupted`
      (`self.K2_EndAbility` :!label _label))
    (:`OnCancelled`
      (goto _label))))