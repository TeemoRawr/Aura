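; BP_FlamePilar is a flame pillar actor that makes its FlameLight flicker continuously.
; On BeginPlay it randomly picks one of two timelines, and picks again whenever the playing one finishes, forming an endless loop.
; Each timeline's FlameIntensity track is multiplied by BaseIntensity to set the light's intensity on every update.
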(event `self.ReceiveBeginPlay`
  (`self.ChooseTimeline`))

(event `ChooseTimeline`
  (switch `int` (`KismetMathLibrary.RandomIntegerInRange` 0 1)
    (:`0`
      (`self.StartTimelineOne`))
    (:`1`
      (`self.StartTimelineTwo`))))

(event `StartTimelineOne`
  (bind (_direction _flameintensity) (`Timeline|TimeIntensityTimelineOne`)
    (:`Update`
      (`self.ScaleFlameIntensity` _flameintensity))
    (:`Finished`
      (`self.ChooseTimeline`))))

(event `StartTimelineTwo`
  (bind (_direction _flameintensity) (`Timeline|TimeIntensityTimelineTwo`)
    (:`Update`
      (`self.ScaleFlameIntensity` _flameintensity))
    (:`Finished`
      (`self.ChooseTimeline`))))

(fn `ScaleFlameIntensity`
  (params (FlameIntensity :type "Float (double-precision)"))
  (`LightComponent.SetIntensity` (`self.FlameLight`) (* FlameIntensity (`self.BaseIntensity`))))

(fn `UserConstructionScript`)